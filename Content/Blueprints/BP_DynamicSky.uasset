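; Dynamic sky actor that sets up time-of-day lighting, atmosphere, clouds and weather from a preset.
; The construction script rotates and toggles sun and moon, then configures stars and sky through a dynamic sky-sphere material.
; Sunny allows 2D or volumetric clouds, while Snowy and Rainy force TimeOfDay to 11.
; Snow drives Niagara and a material parameter collection, with optional timeline-animated coverage from BeginPlay.
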(event EventBeginPlay
  (bind _snowyweathersettings (Variables|04-WeatherSettings|GetSnowyWeatherSettings))
  (bind (_shouldanimatesnowcoverageruntime _fullsnowcoveragetime) (Utilities|Struct|BreakS_SnowyWeatherSettings _snowyweathersettings))
  (04-WeatherSettings|HandleWeatherSettings)
  (Utilities|GetCurrentWeatherType
    (:Snowy
      (if _shouldanimatesnowcoverageruntime
        (Rendering|Material|SetScalarParameterValue "/Game/Materials/MaterialParameterCollection/MPC_WeatherProperties.MPC_WeatherProperties" "SnowAmount" 0.0 :!class /Script/Engine.KismetMaterialLibrary)
        (Utilities|FlowControl|Delay 1.5)
        (Components|Timeline|SetPlayRate (Variables|Default|GetSnowCoverageAnimationTimeline) (/ 1.0 _fullsnowcoveragetime))
        (bind _normalizedfloattrack (Timeline|SnowCoverageAnimationTimeline Play)
          (:Update
            (Rendering|Material|SetScalarParameterValue "/Game/Materials/MaterialParameterCollection/MPC_WeatherProperties.MPC_WeatherProperties" "SnowAmount" _normalizedfloattrack :!class /Script/Engine.KismetMaterialLibrary)))))))

(fn ConstructionScript
  (bind _is_dynmi_skysphere_valid (01-BasicSettings|InitSkySphereMaterial))
  (if _is_dynmi_skysphere_valid
    (Utilities|FlowControl|Sequence
      (:then_0
        (04-WeatherSettings|HandleWeatherSettings))
      (:then_1
        (01-BasicSettings|HandleSunMoonRotation))
      (:then_2
        (01-BasicSettings|HandleVisibility))
      (:then_3
        (02-NightSettings|HandleNightSettings))
      (:then_4
        (03-CloudSettings|HandleCloudSettings)))))

(fn InitSkySphereMaterial
  (bind _returnvalue (Rendering|Material|CreateDynamicMaterialInstance (Variables|Default|GetSM_SkySphere) 0 "/Game/Materials/Sky/MI_DynamicSkySphere.MI_DynamicSkySphere" "None" :!class /Script/Engine.PrimitiveComponent))
  (bind _output_get (Variables|Default|SetCreated_DynMI_SkySphere _returnvalue))
  (return (Utilities|IsValid _output_get)))

(fn HandleSunMoonRotation
  (Transformation|SetWorldRotation (Variables|Default|GetSunDirectionalLight) (Math|Rotator|MakeRotator 0.0 (Math|Float|MapRangeUnclamped (Variables|01-BasicSettings|GetTimeOfDay) (Variables|01-BasicSettings|GetDawnTime) (Variables|01-BasicSettings|GetDuskTime) 0.0 -1.8e+02) (Variables|01-BasicSettings|GetSunMoonRotation)) false false)
  (Transformation|SetWorldRotation (Variables|Default|GetMoonDirectionalLight) (Math|Rotator|MakeRotator 0.0 (Math|Float|MapRangeUnclamped (Variables|01-BasicSettings|GetTimeOfDay) (+ (Variables|01-BasicSettings|GetDuskTime) 0.3) 24.0 -1.8e+02 -9e+01) (Variables|01-BasicSettings|GetSunMoonRotation)) false false)
  (Transformation|SetWorldRotation (Variables|Default|GetMoonDirectionalLight) (Math|Rotator|MakeRotator 0.0 (Math|Float|MapRangeUnclamped (Variables|01-BasicSettings|GetTimeOfDay) 0.0 (- (Variables|01-BasicSettings|GetDawnTime) 0.3) -9e+01 0.0) (Variables|01-BasicSettings|GetSunMoonRotation)) false false))

(fn HandleVisibility
  (Rendering|SetVisibility (Variables|Default|GetSunDirectionalLight) (Utilities|IsDayTime) false)
  (Rendering|SetVisibility (Variables|Default|GetMoonDirectionalLight) (Utilities|IsNightTime) false))

(fn HandleNightSettings
  (if (Utilities|IsNightTime)
    (Utilities|FlowControl|Sequence
      (:then_0
        (Rendering|Components|Light|SetIntensity (Variables|Default|GetMoonDirectionalLight) (Variables|02-NightSettings|GetMoonLightIntensity))
        (Rendering|Components|Light|SetLightColor (Variables|Default|GetMoonDirectionalLight) (Variables|02-NightSettings|GetMoonLightColor) true)
        (Class|DirectionalLightComponent|SetLightSourceAngle (Variables|Default|GetMoonDirectionalLight) (Variables|02-NightSettings|GetMoonLightSourceAngle))
        (Class|LightComponent|SetTemperature (Variables|Default|GetMoonDirectionalLight) (Variables|02-NightSettings|GetMoonLightTemperature)))
      (:then_1
        (Class|SkyAtmosphereComponent|SetRayleighScattering (Variables|Default|GetSkyAtmosphere) (Variables|02-NightSettings|GetNighttimeRaylayScattering))
        (Class|SkyAtmosphereComponent|SetMultiScatteringFactor (Variables|Default|GetSkyAtmosphere) (Variables|02-NightSettings|GetNighttimeMultiScattering)))
      (:then_2
        (Rendering|Material|SetScalarParameterValue (Variables|Default|GetCreated_DynMI_SkySphere) "IsStarVisible" (Math|Float|SelectFloat 1.0 0.0 (Variables|02-NightSettings|GetShouldShowStars)) :!class /Script/Engine.MaterialInstanceDynamic)
        (Rendering|Material|SetScalarParameterValue (Variables|Default|GetCreated_DynMI_SkySphere) "IsMoonVisible" (Math|Float|SelectFloat 1.0 0.0 (Variables|02-NightSettings|GetShouldShowMoon)) :!class /Script/Engine.MaterialInstanceDynamic)
        (Rendering|Material|SetVectorParameterValue (Variables|Default|GetCreated_DynMI_SkySphere) "MoonBasicSettings" (Utilities|Struct|MakeLinearColor (/ (Variables|02-NightSettings|GetMoonScale) 1e+01) (Variables|02-NightSettings|GetMoonStaticRotation) (Variables|02-NightSettings|GetMoonBrightness) 0.0) :!class /Script/Engine.MaterialInstanceDynamic)
        (Rendering|Material|SetVectorParameterValue (Variables|Default|GetCreated_DynMI_SkySphere) "MoonTint" (Variables|02-NightSettings|GetMoonTint) :!class /Script/Engine.MaterialInstanceDynamic)))
    (else
      (04-WeatherSettings|HandleWeatherSettings)
      (Rendering|Material|SetScalarParameterValue (Variables|Default|GetCreated_DynMI_SkySphere) "IsStarVisible" 0.0 :!class /Script/Engine.MaterialInstanceDynamic)
      (Rendering|Material|SetScalarParameterValue (Variables|Default|GetCreated_DynMI_SkySphere) "IsMoonVisible" 0.0 :!class /Script/Engine.MaterialInstanceDynamic))))

(fn HandleCloudSettings
  (Utilities|GetCurrentWeatherType
    (:Sunny
      (switch Utilities|FlowControl|Switch|SwitchonECloudMode (Variables|03-CloudSettings|GetCurrentCloudMode)
        (:NewEnumerator0
          (Utilities|Toggle2DClouds false)
          (Utilities|ToggleVolumetricClouds false))
        (:NewEnumerator1
          (Utilities|Toggle2DClouds true)
          (Utilities|Set2DCloudsSettings)
          (Utilities|ToggleVolumetricClouds false))
        (:NewEnumerator2
          (Utilities|Toggle2DClouds false)
          (Utilities|ToggleVolumetricClouds true)
          (Utilities|SetVolumetricCloudSettings))))
    (:Snowy
      (Utilities|Toggle2DClouds false)
      (Utilities|ToggleVolumetricClouds false))))

(fn HandleWeatherSettings
  (04-WeatherSettings|SetWeatherLightingProperties)
  (Utilities|GetCurrentWeatherType
    (:Sunny
      (Utilities|ToggleSnow false))
    (:Snowy
      (Variables|01-BasicSettings|SetTimeOfDay 11.0)
      (Utilities|ToggleSnow true)
      (Utilities|SetSnowParticleSettings))
    (:Rainy
      (Variables|01-BasicSettings|SetTimeOfDay 11.0)
      (Utilities|ToggleSnow false))))

(fn SetWeatherLightingProperties
  (bind _currentweatherpreset (Variables|04-WeatherSettings|GetCurrentWeatherPreset))
  (bind _currentweatherpreset_2 (Variables|04-WeatherSettings|GetCurrentWeatherPreset))
  (bind _currentweatherpreset_3 (Variables|04-WeatherSettings|GetCurrentWeatherPreset))
  (bind _directionallightsettings (Variables|/Game/DataAssets/BP_WeatherDataAssetBase.BP_WeatherDataAssetBase_C|GetDirectionalLightSettings _currentweatherpreset))
  (bind _skyatmospheresettings (Variables|/Game/DataAssets/BP_WeatherDataAssetBase.BP_WeatherDataAssetBase_C|GetSkyAtmosphereSettings _currentweatherpreset_2))
  (bind _exponentialheightfogsettings (Variables|/Game/DataAssets/BP_WeatherDataAssetBase.BP_WeatherDataAssetBase_C|GetExponentialHeightFogSettings _currentweatherpreset_3))
  (bind (_dirlightintensity _dirlightcolor _dirlightsourceangle _temperature) (Utilities|Struct|BreakS_DirectionalLightSettings _directionallightsettings))
  (bind (_multiscattering _rayleighscattering _miescatteringscale _mieabsorptionscale _mieanisotropy _aerialperspectiveviewdistancescale) (Utilities|Struct|BreakS_SkyAtmosphereSettings _skyatmospheresettings))
  (bind (_emissive _extinctionscale) (Utilities|Struct|BreakS_ExponentialHeightFogFog _exponentialheightfogsettings))
  (if (Utilities|IsDayTime)
    (Utilities|FlowControl|Sequence
      (:then_0
        (Rendering|Components|Light|SetIntensity (Variables|Default|GetSunDirectionalLight) _dirlightintensity)
        (Rendering|Components|Light|SetLightColor (Variables|Default|GetSunDirectionalLight) _dirlightcolor true)
        (Class|DirectionalLightComponent|SetLightSourceAngle (Variables|Default|GetSunDirectionalLight) _dirlightsourceangle)
        (Class|LightComponent|SetTemperature (Variables|Default|GetSunDirectionalLight) _temperature))
      (:then_1
        (Rendering|Components|Light|SetIntensity (Variables|Default|GetSkyLight) (Utilities|Struct|BreakS_SkyLight_Settings (Variables|/Game/DataAssets/BP_WeatherDataAssetBase.BP_WeatherDataAssetBase_C|GetSkyLightSettings (Variables|04-WeatherSettings|GetCurrentWeatherPreset)))))
      (:then_2
        (Class|SkyAtmosphereComponent|SetMultiScatteringFactor (Variables|Default|GetSkyAtmosphere) _multiscattering)
        (Class|SkyAtmosphereComponent|SetRayleighScattering (Variables|Default|GetSkyAtmosphere) _rayleighscattering)
        (Class|SkyAtmosphereComponent|SetMieScatteringScale (Variables|Default|GetSkyAtmosphere) _miescatteringscale)
        (Class|SkyAtmosphereComponent|SetMieAbsorptionScale (Variables|Default|GetSkyAtmosphere) _mieabsorptionscale)
        (Class|SkyAtmosphereComponent|SetMieAnisotropy (Variables|Default|GetSkyAtmosphere) _mieanisotropy)
        (Class|SkyAtmosphereComponent|SetAerialPespectiveViewDistanceScale (Variables|Default|GetSkyAtmosphere) _aerialperspectiveviewdistancescale))
      (:then_3
        (Class|ExponentialHeightFogComponent|SetVolumetricFogEmissive (Variables|Default|GetExponentialHeightFog) _emissive)
        (Class|ExponentialHeightFogComponent|SetVolumetricFogExtinctionScale (Variables|Default|GetExponentialHeightFog) _extinctionscale)))))